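; Door obstacle that slides its Plane back and forth between StartPoint and EndPoint, starting at BeginPlay.
; The Travel timeline lerps the Plane's relative location without sweep, at a play rate equal to the inverse of DoorSpeed.
; Each time the timeline finishes, RestartTimeLine uses a toggled Flag to play from start or reverse from end, keeping the motion looping.
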(event EventBeginPlay
  (Utilities|FlowControl|Sequence
    (:then_0
      (Components|Timeline|SetPlayRate (Variables|Default|GetTravel) (/ 1.0 (Variables|Default|GetDoorSpeed))))
    (:then_1
      (bind _newtrack_0 (Timeline|Travel Play)
        (:Update
          (Transformation|SetRelativeLocation (Variables|Default|GetPlane) (Math|Vector|Lerp(Vector) (Variables|/Script/Engine.SceneComponent|GetRelativeLocation (Variables|Default|GetStartPoint)) (Variables|/Script/Engine.SceneComponent|GetRelativeLocation (Variables|Default|GetEndPoint)) _newtrack_0) false false))
        (:Finished
          (CallFunction|RestartTimeLine))))))

(fn ConstructionScript)

(fn RestartTimeLine
  (if (Variables|Default|GetFlag)
    (Components|Timeline|PlayfromStart (Variables|Default|GetTravel))
    (Variables|Default|SetFlag false)
    (else
      (Components|Timeline|ReversefromEnd (Variables|Default|GetTravel))
      (Variables|Default|SetFlag true))))