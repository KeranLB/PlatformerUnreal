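; BP_wind is an environment wind volume that launches the third-person character when it enters the box.
; On overlap, it resets the character's movement gravity scale to normal, then launches it along the DirectionWind0 forward vector scaled by WindForce, overriding existing velocity.
; After a short delay, it lowers gravity scale again if the character's IsPlaning flag is set, apparently resuming a glide.
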(event OnComponentBeginOverlap(Box)
  (params (OverlappedComponent :type Primitive%20Component%20Object%20Reference) (OtherActor :type Actor%20Object%20Reference) (OtherComp :type Primitive%20Component%20Object%20Reference) (OtherBodyIndex :type Integer) (bFromSweep :type Boolean) (SweepResult :type Hit%20Result%20Structure%20%28by%20ref%29))
  (bind _returnvalue (Actor|GetComponentbyClass OtherActor "/Script/Engine.CharacterMovementComponent"))
  (Variables|/Script/Engine.CharacterMovementComponent|SetGravityScale _returnvalue 1.0)
  (bind _asbp_third_person_character (Utilities|Casting|CastToBP_ThirdPersonCharacter (Components|GetOwner _returnvalue)))
  (Character|LaunchCharacter _asbp_third_person_character (* (Math|Vector|GetForwardVector (Variables|Default|GetDirectionWind_0)) (Variables|Default|GetWindForce)) true true)
  (Utilities|FlowControl|Delay 1.0)
  (if (Variables|/Game/ThirdPerson/Blueprints/BP_ThirdPersonCharacter.BP_ThirdPersonCharacter_C|GetisPlaning _asbp_third_person_character)
    (Variables|/Script/Engine.CharacterMovementComponent|SetGravityScale _returnvalue 0.1)))

(fn ConstructionScript)