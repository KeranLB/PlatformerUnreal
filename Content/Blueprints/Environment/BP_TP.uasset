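; BP_TP is a key-unlocked teleporter that sends the player to a checkpoint.
; On BeginPlay it disables overlap events on its Box and hides its Plane.
; A hit on the Key component enables the Box, reveals the Plane and destroys the Key.
; Box overlaps then cast the overlapping actor's owner to BP_MyThirdPersonPlayerController and call Respawn with the CheckPoint variable.
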(event OnComponentBeginOverlap(Box)
  (params (OverlappedComponent :type Primitive%20Component%20Object%20Reference) (OtherActor :type Actor%20Object%20Reference) (OtherComp :type Primitive%20Component%20Object%20Reference) (OtherBodyIndex :type Integer) (bFromSweep :type Boolean) (SweepResult :type Hit%20Result%20Structure%20%28by%20ref%29))
  (bind _asbp_my_third_person_player_controller (Utilities|Casting|CastToBP_MyThirdPersonPlayerController (Components|GetOwner OtherActor)))
  (Default|Respawn _asbp_my_third_person_player_controller (Variables|Default|GetCheckPoint)))

(event OnComponentHit(Key)
  (params (HitComponent :type Primitive%20Component%20Object%20Reference) (OtherActor :type Actor%20Object%20Reference) (OtherComp :type Primitive%20Component%20Object%20Reference) (NormalImpulse :type Vector :default "0, 0, 0") (Hit :type Hit%20Result%20Structure%20%28by%20ref%29))
  (Variables|/Script/Engine.PrimitiveComponent|SetbGenerateOverlapEvents (Variables|Default|GetBox) true)
  (Rendering|SetVisibility (Variables|Default|GetPlane) true false)
  (Components|DestroyComponent (Variables|Default|GetKey)))

(event EventBeginPlay
  (Variables|/Script/Engine.PrimitiveComponent|SetbGenerateOverlapEvents (Variables|Default|GetBox) false)
  (Rendering|SetVisibility (Variables|Default|GetPlane) false false))

(event Collision|EventActorBeginOverlap
  (params (OtherActor :type Actor%20Object%20Reference)))

(event EventTick
  (params (DeltaSeconds :type Float%20%28single-precision%29)))

(fn ConstructionScript)